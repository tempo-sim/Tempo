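; PCG grass actor, named for GPU generation, that uses a scene capture to define where grass is excluded.
; RefreshGrassExclusion appends actors matching configured tags and classes to an exclusion list, then captures only those actors.
; It then refreshes the runtime PCG component without flushing its cache and resets the capture's show-only list.
; The event graph and construction script are empty.
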(event EventBeginPlay)

(event Collision|EventActorBeginOverlap
  (params (OtherActor :type Actor%20Object%20Reference)))

(event EventTick
  (params (DeltaSeconds :type Float%20%28single-precision%29)))

(fn ConstructionScript)

(fn RefreshGrassExclusion
  (bind _valuepin (Utilities|Set|ForEachLoop(Set) (Variables|Default|GetGrassExclusionActorTags))
    (:then
      (bind _outactors (Actor|GetAllActorswithTag _valuepin))
      (Utilities|Array|AppendArray (LocalVariables|GetGrassExclusionActors) _outactors))
    (:CompletedPin
      (bind _valuepin_2 (Utilities|Set|ForEachLoop(Set) (Variables|Default|GetGrassExclusionActorClasses))
        (:then
          (bind _outactors_2 (Actor|GetAllActorsOfClass _valuepin_2))
          (Utilities|Array|AppendArray (LocalVariables|GetGrassExclusionActors) _outactors_2))
        (:CompletedPin
          (Variables|/Script/Engine.SceneCaptureComponent|SetShowOnlyActors (Variables|Default|GetGrassExclusionCaptureComponent) (LocalVariables|GetGrassExclusionActors))
          (Rendering|SceneCapture|CaptureScene (Variables|Default|GetGrassExclusionCaptureComponent) :!class /Script/Engine.SceneCaptureComponent2D)
          (Class|PCGBlueprintHelpers|RefreshPCGRuntimeComponent (Variables|Default|GetPCG) false)
          (Variables|/Script/Engine.SceneCaptureComponent|SetShowOnlyActors (Variables|Default|GetGrassExclusionCaptureComponent) (Utilities|Array|MakeArray 0)))))))