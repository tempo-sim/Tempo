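; BP_IntersectionProxy is an actor representing an intersection of up to four connected roads for the Tempo traffic system.
; It answers Tempo interface queries for entrances, lane filtering and controller placement by forwarding to TempoIntersectionQuery and TempoIntersectionControl components.
; On setup, it assigns three- or four-way sign layouts rotated to a canonical starting connection, then builds controllers using sign or traffic-light meshes.
; The entrance tangent getter also draws a debug arrow.
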(event `self.SetupTempoTrafficControllers`
  (`self.SetupTrafficSignTypes`)
  (`TempoIntersectionControlComponent.SetupTrafficControllers` (`self.TempoIntersectionControl`)))

(fn `GetConnectedTempoRoadActor`
  (params (ConnectionIndex :type Integer))
  (returns (ReturnValue :type "Actor Object Reference"))
  (switch `int` ConnectionIndex
    (:`0`
      (return (`self.ConnectedRoad1`)))
    (:`1`
      (return (`self.ConnectedRoad2`)))
    (:`2`
      (return (`self.ConnectedRoad3`)))
    (:`3`
      (return (`self.ConnectedRoad4`)))))

(fn `GetConnectedTempoRoadModuleActor`
  (params (ConnectedRoadModuleIndex :type Integer))
  (returns (ReturnValue :type "Actor Object Reference"))
  (return null))

(fn `GetNumConnectedTempoRoadModules`
  (returns (ReturnValue :type Integer))
  (return 0))

(fn `GetNumTempoConnections`
  (returns (ReturnValue :type Integer))
  (locals (ValidConnectedRoads :type "Set of Actor Object Reference"))
  (bind _connectedroad3 (`self.ConnectedRoad3`))
  (bind _connectedroad1 (`self.ConnectedRoad1`))
  (bind _connectedroad2 (`self.ConnectedRoad2`))
  (bind _connectedroad4 (`self.ConnectedRoad4`))
  (`/Engine/EditorBlueprintResources/StandardMacros.IsValid` _connectedroad1
    (:`Is Valid`
      (`BlueprintSetLibrary.Set_Add` (`local.ValidConnectedRoads`) _connectedroad1))
    (:`Is Not Valid`
      _))
  (`/Engine/EditorBlueprintResources/StandardMacros.IsValid` _connectedroad2
    (:`Is Valid`
      (`BlueprintSetLibrary.Set_Add` (`local.ValidConnectedRoads`) _connectedroad2))
    (:`Is Not Valid`
      _))
  (`/Engine/EditorBlueprintResources/StandardMacros.IsValid` _connectedroad3
    (:`Is Valid`
      (`BlueprintSetLibrary.Set_Add` (`local.ValidConnectedRoads`) _connectedroad3))
    (:`Is Not Valid`
      _))
  (`/Engine/EditorBlueprintResources/StandardMacros.IsValid` _connectedroad4
    (:`Is Valid`
      (`BlueprintSetLibrary.Set_Add` (`local.ValidConnectedRoads`) _connectedroad4))
    (:`Is Not Valid`
      _))
  (return (`BlueprintSetLibrary.Set_Length` (`local.ValidConnectedRoads`))))

(fn `GetTempoIntersectionEntranceControlPointIndex`
  (params (ConnectionIndex :type Integer))
  (returns (ReturnValue :type Integer))
  (bind (_outintersectionentrancecontrolpointindex _returnvalue) (`TempoIntersectionQueryComponent.TryGetIntersectionEntranceControlPointIndex` (`self.TempoIntersectionQuery`) self ConnectionIndex))
  (if _returnvalue
    (return _outintersectionentrancecontrolpointindex)
    (else
      (return -1))))

(fn `GetTempoIntersectionEntranceLocation`
  (params (ConnectionIndex :type Integer) (CoordinateSpace :type "ETempoCoordinateSpace Enum" :default "Local"))
  (returns (ReturnValue :type "Vector Structure"))
  (bind (_outintersectionentrancelocation _returnvalue) (`TempoIntersectionQueryComponent.TryGetIntersectionEntranceLocation` (`self.TempoIntersectionQuery`) self ConnectionIndex CoordinateSpace))
  (if _returnvalue
    (return _outintersectionentrancelocation)
    (else
      (return (0.0 0.0 0.0)))))

(fn `GetTempoIntersectionEntranceRightVector`
  (params (ConnectionIndex :type Integer) (CoordinateSpace :type "ETempoCoordinateSpace Enum" :default "Local"))
  (returns (ReturnValue :type "Vector Structure"))
  (locals (Float :type "Float (double-precision)" :default 1000.0))
  (bind (_outintersectionentrancerightvector _returnvalue) (`TempoIntersectionQueryComponent.TryGetIntersectionEntranceRightVector` (`self.TempoIntersectionQuery`) self ConnectionIndex CoordinateSpace))
  (if _returnvalue
    (return _outintersectionentrancerightvector)
    (else
      (return (0.0 0.0 0.0)))))

(fn `GetTempoIntersectionEntranceTangent`
  (params (ConnectionIndex :type Integer) (CoordinateSpace :type "ETempoCoordinateSpace Enum" :default "Local"))
  (returns (ReturnValue :type "Vector Structure"))
  (locals (Float :type "Float (double-precision)" :default 500.0))
  (bind _tempointersectionquery (`self.TempoIntersectionQuery`))
  (bind (_outintersectionentrancetangent _returnvalue) (`TempoIntersectionQueryComponent.TryGetIntersectionEntranceTangent` _tempointersectionquery self ConnectionIndex CoordinateSpace))
  (bind _outintersectionentrancelocation (`TempoIntersectionQueryComponent.TryGetIntersectionEntranceLocation` _tempointersectionquery self ConnectionIndex CoordinateSpace))
  (if _returnvalue
    (`KismetSystemLibrary.DrawDebugArrow` _outintersectionentrancelocation (+ _outintersectionentrancelocation (* _outintersectionentrancetangent (`local.Float`))) 100.0 (struct :`G` 1.0 :`B` 0.126716 :`A` 1.0) 10.0 10.0)
    (return _outintersectionentrancetangent)
    (else
      (return (0.0 0.0 0.0)))))

(fn `GetTempoIntersectionEntranceUpVector`
  (params (ConnectionIndex :type Integer) (CoordinateSpace :type "ETempoCoordinateSpace Enum" :default "Local"))
  (returns (ReturnValue :type "Vector Structure"))
  (locals (Float :type "Float (double-precision)" :default 1000.0))
  (bind (_outintersectionentranceupvector _returnvalue) (`TempoIntersectionQueryComponent.TryGetIntersectionEntranceUpVector` (`self.TempoIntersectionQuery`) self ConnectionIndex CoordinateSpace))
  (if _returnvalue
    (return _outintersectionentranceupvector)
    (else
      (return (0.0 0.0 0.0)))))

(fn `GetTempoIntersectionTags`
  (returns (ReturnValue :type "Array of Name"))
  (return (`|MakeArray` "Intersection" :!type "Name")))

(fn `GetTempoRoadConfigurationInfo`
  (params (SourceConnectionIndex :type Integer) (RoadConfigurationDescriptor :type "ETempoRoadConfigurationDescriptor Enum" :default "ThroughRoad"))
  (returns (ReturnValue :type "Array of TempoRoadConfigurationInfo Structure"))
  (bind (_outroadconfigurationinfos _returnvalue) (`TempoIntersectionControlComponent.TryGetRoadConfigurationInfoForIntersection` (`self.TempoIntersectionControl`) self SourceConnectionIndex RoadConfigurationDescriptor))
  (if _returnvalue
    (return _outroadconfigurationinfos)
    (else
      (return))))

(fn `GetTempoTrafficControllerLocation`
  (params (ConnectionIndex :type Integer) (TrafficControllerType :type "ETempoTrafficControllerType Enum" :default "Sign") (CoordinateSpace :type "ETempoCoordinateSpace Enum" :default "Local"))
  (returns (ReturnValue :type "Vector Structure"))
  (bind (_outintersectiontrafficcontrollerlocation _returnvalue) (`TempoIntersectionControlComponent.TryGetIntersectionTrafficControllerLocation` (`self.TempoIntersectionControl`) self ConnectionIndex TrafficControllerType (`self.GetTrafficControllerMeshInfo` ConnectionIndex) CoordinateSpace))
  (if _returnvalue
    (return _outintersectiontrafficcontrollerlocation)
    (else
      (return (0.0 0.0 0.0)))))

(fn `GetTempoTrafficControllerMeshInfo`
  (params (ConnectionIndex :type Integer) (TrafficControllerType :type "ETempoTrafficControllerType Enum" :default "Sign"))
  (returns (ReturnValue :type "TempoTrafficControllerMeshInfo Structure"))
  (return (`self.GetTrafficControllerMeshInfo` ConnectionIndex)))

(fn `GetTempoTrafficControllerRotation`
  (params (ConnectionIndex :type Integer) (TrafficControllerType :type "ETempoTrafficControllerType Enum" :default "Sign") (CoordinateSpace :type "ETempoCoordinateSpace Enum" :default "Local"))
  (returns (ReturnValue :type "Rotator Structure"))
  (bind (_outintersectiontrafficcontrollerrotation _returnvalue) (`TempoIntersectionControlComponent.TryGetIntersectionTrafficControllerRotation` (`self.TempoIntersectionControl`) self ConnectionIndex TrafficControllerType (`self.GetTrafficControllerMeshInfo` ConnectionIndex) CoordinateSpace))
  (if _returnvalue
    (return _outintersectiontrafficcontrollerrotation)
    (else
      (return))))

(fn `GetTempoTrafficControllerSignType`
  (params (ConnectionIndex :type Integer))
  (returns (ReturnValue :type "EMassTrafficControllerSignType Enum"))
  (return (`|GetArrayItem` (`self.TrafficControllerSignType`) (mod ConnectionIndex (`KismetArrayLibrary.Array_Length` (`self.TrafficControllerSignType`))))))

(fn `GetTempoTrafficControllerType`
  (returns (ReturnValue :type "ETempoTrafficControllerType Enum"))
  (return (`self.TrafficControllerType`)))

(fn `GetTrafficControllerMeshInfo`
  (params (ConnectionIndex :type Integer))
  (returns (ReturnValue :type "TempoTrafficControllerMeshInfo Structure"))
  (return (`|GetArrayItem` (`self.GetTrafficControllerMeshInfos` ConnectionIndex) (mod ConnectionIndex (`KismetArrayLibrary.Array_Length` (`self.GetTrafficControllerMeshInfos` ConnectionIndex))))))

(fn `GetTrafficControllerMeshInfos`
  (params (ConnectionIndex :type Integer))
  (returns (ReturnValue :type "Array of TempoTrafficControllerMeshInfo Structure"))
  (switch `ETempoTrafficControllerType` (`self.GetTrafficControllerType`)
    (:`Sign`
      (switch `EMassTrafficControllerSignType` (`self.GetTempoTrafficControllerSignType` ConnectionIndex)
        (:`None`
          (return))
        (:`YieldSign`
          (return (`self.TrafficController_YieldSignMeshInfo`)))
        (:`StopSign`
          (return (`self.TrafficController_StopSignMeshInfo`)))))
    (:`TrafficLight`
      (return (`self.TrafficController_TrafficLightMeshInfo`)))))

(fn `GetTrafficControllerType`
  (returns (ReturnValue :type "ETempoTrafficControllerType Enum"))
  (return (`self.TrafficControllerType`)))

(fn `SetupTrafficSignTypes`
  (locals (StartingConnectionIndexLocal :type Integer :default 0) (SignTypeConfigurationLocal :type "Array of EMassTrafficControllerSignType Enum"))
  (bind _returnvalue (`self.GetNumTempoConnections`))
  (bind (_outstartingconnectionindex _returnvalue_2) (`TempoIntersectionQueryComponent.TryGetCanonicalStartingConnectionIndex` (`self.TempoIntersectionQuery`) self))
  (if (or (== _returnvalue 3) (== _returnvalue 4))
    (switch `int` (`self.GetNumTempoConnections`)
      (:`3`
        (set `local.SignTypeConfigurationLocal` (`self.ThreeSidedSignTypeConfiguration`)))
      (:`4`
        (set `local.SignTypeConfigurationLocal` (`self.FourSidedSignTypeConfiguration`))))
    (`KismetArrayLibrary.Array_Clear` (`self.TrafficControllerSignType`))
    (`KismetArrayLibrary.Array_Resize` (`self.TrafficControllerSignType`) (`KismetArrayLibrary.Array_Length` (`local.SignTypeConfigurationLocal`)))
    (if _returnvalue_2
      (set `local.StartingConnectionIndexLocal` _outstartingconnectionindex)
      (for _index (range (`self.GetNumTempoConnections`))
        (`KismetArrayLibrary.Array_Set` (`self.TrafficControllerSignType`) (mod (+ _index (`local.StartingConnectionIndexLocal`)) (`self.GetNumTempoConnections`)) (`|GetArrayItem` (`local.SignTypeConfigurationLocal`) _index))))))

(fn `ShouldFilterTempoLaneConnection`
  (params (SourceConnectionActor :type "Actor Object Reference") (SourceLaneConnectionInfos :type "Array of TempoLaneConnectionInfo Structure (by ref)") (SourceSlotQueryIndex :type Integer) (DestConnectionActor :type "Actor Object Reference") (DestLaneConnectionInfos :type "Array of TempoLaneConnectionInfo Structure (by ref)") (DestSlotQueryIndex :type Integer) (AllCandidates :type "Array of LaneConnectionCandidate Structure (by ref)"))
  (returns (ReturnValue :type Boolean))
  (return (`TempoIntersectionQueryComponent.ShouldFilterLaneConnection` (`self.TempoIntersectionQuery`) SourceConnectionActor SourceLaneConnectionInfos SourceSlotQueryIndex DestConnectionActor DestLaneConnectionInfos DestSlotQueryIndex AllCandidates)))

(fn `Spawn All Roads`)

(fn `UserConstructionScript`)