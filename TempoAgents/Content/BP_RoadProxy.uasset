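; BP_RoadProxy is a spline-based stand-in road that answers Tempo road queries for geometry, lanes and zone shape generation.
; Getters read the Spline and lane variables, expose left and right child-actor road modules, and stub out parking.
; The construction script can snap spline points to ground via vertical traces that ignore procedural foliage volumes.
; The last lane runs forward, all others backward, and total width counts the left shoulder twice.
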(fn `GetConnectedTempoRoadModuleActor`
  (params (ConnectedRoadModuleIndex :type Integer))
  (returns (ReturnValue :type "Actor Object Reference"))
  (switch `int` ConnectedRoadModuleIndex
    (:`0`
      (return (`ChildActorComponent.ChildActor` (`self.RoadModuleLeft`))))
    (:`1`
      (return (`ChildActorComponent.ChildActor` (`self.RoadModuleRight`))))))

(fn `GetDistanceAlongTempoRoadAtControlPoint`
  (params (ControlPointIndex :type Integer))
  (returns (ReturnValue :type "Float (single-precision)"))
  (return (`SplineComponent.GetDistanceAlongSplineAtSplinePoint` (`self.Spline`) ControlPointIndex)))

(fn `GetDistanceAlongTempoRoadClosestToWorldLocation`
  (params (QueryLocation :type "Vector Structure"))
  (returns (ReturnValue :type "Float (single-precision)"))
  (bind _returnvalue (message `TempoRoadInterface.GetDistanceAlongTempoRoadClosestToWorldLocation` (`self.Spline`) QueryLocation))
  (return _returnvalue))

(fn `GetEntityTypesAllowedToParkOnTempoRoad`
  (returns (ReturnValue :type "Set of MassEntityConfigAsset Soft Object Reference"))
  (return))

(fn `GetLocationAtDistanceAlongTempoRoad`
  (params (DistanceAlongRoad :type "Float (single-precision)") (CoordinateSpace :type "ETempoCoordinateSpace Enum" :default "Local"))
  (returns (ReturnValue :type "Vector Structure"))
  (bind _spline (`self.Spline`))
  (switch `ETempoCoordinateSpace` CoordinateSpace
    (:`Local`
      (return (`SplineComponent.GetLocationAtDistanceAlongSpline` _spline DistanceAlongRoad "Local")))
    (:`World`
      (return (`SplineComponent.GetLocationAtDistanceAlongSpline` _spline DistanceAlongRoad "World")))))

(fn `GetMaxAllowedParkingSpawnPointsOnTempoRoad`
  (returns (ReturnValue :type Integer))
  (return 0))

(fn `GetNumConnectedTempoRoadModules`
  (returns (ReturnValue :type Integer))
  (return 2))

(fn `GetNumTempoControlPoints`
  (returns (ReturnValue :type Integer))
  (return (`SplineComponent.GetNumberOfSplinePoints` (`self.Spline`))))

(fn `GetNumTempoLanes`
  (returns (ReturnValue :type Integer))
  (return (`self.NumLanes`)))

(fn `GetRightVectorAtDistanceAlongTempoRoad`
  (params (DistanceAlongRoad :type "Float (single-precision)") (CoordinateSpace :type "ETempoCoordinateSpace Enum" :default "Local"))
  (returns (ReturnValue :type "Vector Structure"))
  (bind _spline (`self.Spline`))
  (switch `ETempoCoordinateSpace` CoordinateSpace
    (:`Local`
      (return (`SplineComponent.GetRightVectorAtDistanceAlongSpline` _spline DistanceAlongRoad "Local")))
    (:`World`
      (return (`SplineComponent.GetRightVectorAtDistanceAlongSpline` _spline DistanceAlongRoad "World")))))

(fn `GetRotationAtDistanceAlongTempoRoad`
  (params (DistanceAlongRoad :type "Float (single-precision)") (CoordinateSpace :type "ETempoCoordinateSpace Enum" :default "Local"))
  (returns (ReturnValue :type "Rotator Structure"))
  (bind _spline (`self.Spline`))
  (switch `ETempoCoordinateSpace` CoordinateSpace
    (:`Local`
      (return (`SplineComponent.GetRotationAtDistanceAlongSpline` _spline DistanceAlongRoad "Local")))
    (:`World`
      (return (`SplineComponent.GetRotationAtDistanceAlongSpline` _spline DistanceAlongRoad "World")))))

(fn `GetTangentAtDistanceAlongTempoRoad`
  (params (DistanceAlongRoad :type "Float (single-precision)") (CoordinateSpace :type "ETempoCoordinateSpace Enum" :default "Local"))
  (returns (ReturnValue :type "Vector Structure"))
  (bind _spline (`self.Spline`))
  (switch `ETempoCoordinateSpace` CoordinateSpace
    (:`Local`
      (return (`SplineComponent.GetTangentAtDistanceAlongSpline` _spline DistanceAlongRoad "Local")))
    (:`World`
      (return (`SplineComponent.GetTangentAtDistanceAlongSpline` _spline DistanceAlongRoad "World")))))

(fn `GetTempoControlPointLocation`
  (params (ControlPointIndex :type Integer) (CoordinateSpace :type "ETempoCoordinateSpace Enum" :default "Local"))
  (returns (ReturnValue :type "Vector Structure"))
  (bind _spline (`self.Spline`))
  (switch `ETempoCoordinateSpace` CoordinateSpace
    (:`Local`
      (return (`SplineComponent.GetLocationAtSplinePoint` _spline ControlPointIndex "Local")))
    (:`World`
      (return (`SplineComponent.GetLocationAtSplinePoint` _spline ControlPointIndex "World")))))

(fn `GetTempoControlPointRightVector`
  (params (ControlPointIndex :type Integer) (CoordinateSpace :type "ETempoCoordinateSpace Enum" :default "Local"))
  (returns (ReturnValue :type "Vector Structure"))
  (bind _spline (`self.Spline`))
  (switch `ETempoCoordinateSpace` CoordinateSpace
    (:`Local`
      (return (`SplineComponent.GetRightVectorAtSplinePoint` _spline ControlPointIndex "Local")))
    (:`World`
      (return (`SplineComponent.GetRightVectorAtSplinePoint` _spline ControlPointIndex "World")))))

(fn `GetTempoControlPointRotation`
  (params (ControlPointIndex :type Integer) (CoordinateSpace :type "ETempoCoordinateSpace Enum" :default "Local"))
  (returns (ReturnValue :type "Rotator Structure"))
  (bind _spline (`self.Spline`))
  (switch `ETempoCoordinateSpace` CoordinateSpace
    (:`Local`
      (return (`SplineComponent.GetRotationAtSplinePoint` _spline ControlPointIndex "Local")))
    (:`World`
      (return (`SplineComponent.GetRotationAtSplinePoint` _spline ControlPointIndex "World")))))

(fn `GetTempoControlPointTangent`
  (params (ControlPointIndex :type Integer) (CoordinateSpace :type "ETempoCoordinateSpace Enum" :default "Local"))
  (returns (ReturnValue :type "Vector Structure"))
  (bind _spline (`self.Spline`))
  (switch `ETempoCoordinateSpace` CoordinateSpace
    (:`Local`
      (return (`SplineComponent.GetTangentAtSplinePoint` _spline ControlPointIndex "Local")))
    (:`World`
      (return (`SplineComponent.GetTangentAtSplinePoint` _spline ControlPointIndex "World")))))

(fn `GetTempoControlPointUpVector`
  (params (ControlPointIndex :type Integer) (CoordinateSpace :type "ETempoCoordinateSpace Enum" :default "Local"))
  (returns (ReturnValue :type "Vector Structure"))
  (bind _spline (`self.Spline`))
  (switch `ETempoCoordinateSpace` CoordinateSpace
    (:`Local`
      (return (`/TempoAgents/Utilities/SplineFunctionLibrary.GetTempoControlPointUpVector` _spline ControlPointIndex)))
    (:`World`
      (return (`/TempoAgents/Utilities/SplineFunctionLibrary.GetTempoControlPointUpVector` _spline ControlPointIndex "World")))))

(fn `GetTempoEndEntranceLocationControlPointIndex`
  (returns (ReturnValue :type Integer))
  (return (- (`SplineComponent.GetNumberOfSplinePoints` (`self.Spline`)) 1)))

(fn `GetTempoLaneConnectionAllTags`
  (params (LaneIndex :type Integer))
  (returns (ReturnValue :type "Array of Name"))
  (return))

(fn `GetTempoLaneConnectionAnyTags`
  (params (LaneIndex :type Integer))
  (returns (ReturnValue :type "Array of Name"))
  (return))

(fn `GetTempoLaneConnectionNotTags`
  (params (LaneIndex :type Integer))
  (returns (ReturnValue :type "Array of Name"))
  (return))

(fn `GetTempoLaneDirection`
  (params (LaneIndex :type Integer))
  (returns (ReturnValue :type "EZoneLaneDirection Enum"))
  (if (>= LaneIndex (- (`self.GetNumTempoLanes`) 1))
    (return "Forward")
    (else
      (return "Backward"))))

(fn `GetTempoLaneProfileOverrideName`
  (returns (ReturnValue :type Name))
  (return "None"))

(fn `GetTempoLaneTags`
  (params (LaneIndex :type Integer))
  (returns (ReturnValue :type "Array of Name"))
  (return (`|MakeArray` "DrivingLane" :!type "Name")))

(fn `GetTempoLaneWidth`
  (params (LaneIndex :type Integer))
  (returns (ReturnValue :type "Float (single-precision)"))
  (return (`self.LaneWidth`)))

(fn `GetTempoParkingLocation`
  (params (ParkingLocationAnchorName :type Name) (NormalizedDistanceAlongRoad :type "Float (single-precision)") (HalfWidth :type "Float (single-precision)") (NormalizedLateralVariationScalar :type "Float (single-precision)") (CoordinateSpace :type "ETempoCoordinateSpace Enum" :default "Local"))
  (returns (ReturnValue :type "Vector Structure"))
  (return (0.0 0.0 0.0)))

(fn `GetTempoParkingLocationAnchorNames`
  (returns (ReturnValue :type "Array of Name"))
  (return))

(fn `GetTempoParkingRotation`
  (params (ParkingLocationAnchorName :type Name) (NormalizedDistanceAlongRoad :type "Float (single-precision)") (NormalizedAngularVariationScalar :type "Float (single-precision)") (CoordinateSpace :type "ETempoCoordinateSpace Enum" :default "Local"))
  (returns (ReturnValue :type "Rotator Structure"))
  (return))

(fn `GetTempoRoadSampleDistanceStepSize`
  (returns (ReturnValue :type "Float (single-precision)"))
  (return (`self.SampleDistanceStepSize`)))

(fn `GetTempoRoadShoulderWidth`
  (params (LateralSide :type "ETempoRoadLateralDirection Enum" :default "Left"))
  (returns (ReturnValue :type "Float (single-precision)"))
  (return (`self.ShoulderWidth`)))

(fn `GetTempoRoadWidth`
  (returns (ReturnValue :type "Float (single-precision)"))
  (locals (Width :type "Float (double-precision)"))
  (for _index (range (`self.GetNumTempoLanes`))
    (set `local.Width` (+ (`self.GetTempoLaneWidth` _index) (`local.Width`))))
  (bind _output_get (set `local.Width` (+ (`local.Width`) (`self.GetTempoRoadShoulderWidth` "Left") (`self.GetTempoRoadShoulderWidth` "Left"))))
  (return _output_get))

(fn `GetTempoStartEntranceLocationControlPointIndex`
  (returns (ReturnValue :type Integer))
  (return 0))

(fn `GetUpVectorAtDistanceAlongTempoRoad`
  (params (DistanceAlongRoad :type "Float (single-precision)") (CoordinateSpace :type "ETempoCoordinateSpace Enum" :default "Local"))
  (returns (ReturnValue :type "Vector Structure"))
  (bind _spline (`self.Spline`))
  (switch `ETempoCoordinateSpace` CoordinateSpace
    (:`Local`
      (return (`SplineComponent.GetUpVectorAtDistanceAlongSpline` _spline DistanceAlongRoad "Local")))
    (:`World`
      (return (`SplineComponent.GetUpVectorAtDistanceAlongSpline` _spline DistanceAlongRoad "World")))))

(fn `IsTempoLaneClosedLoop`
  (returns (ReturnValue :type Boolean))
  (return false))

(fn `ShouldGenerateZoneShapesForTempoRoad`
  (returns (ReturnValue :type Boolean))
  (return true))

(fn `ShouldSpawnParkedVehiclesForTempoRoad`
  (returns (ReturnValue :type Boolean))
  (return false))

(fn `SnapSplineToGround`
  (locals (ActorsToIgnore :type "Array of Actor Object Reference"))
  (bind _spline (`self.Spline`))
  (bind _groundsearchdist (`self.GroundSearchDist`))
  (if (not (`SplineComponent.bInputSplinePointsToConstructionScript` (`self.Spline`)))
    (`KismetSystemLibrary.PrintString` (`KismetTextLibrary.Conv_TextToString` (`|FormatText` "Spline component on {actor} not set to input spline points to construction script - ground snap will not work" (`KismetSystemLibrary.GetDisplayName` self))))
    (else
      (bind _outactors (`GameplayStatics.GetAllActorsOfClass` "/Script/Foliage.ProceduralFoliageVolume"))
      (set `local.ActorsToIgnore` _outactors)
      (for _index (range (`SplineComponent.GetNumberOfSplinePoints` _spline))
        (bind _returnvalue (`SplineComponent.GetLocationAtSplinePoint` _spline _index "World"))
        (bind _outhit (`KismetSystemLibrary.LineTraceSingleForObjects` (+ _returnvalue (`KismetMathLibrary.MakeVector` 0.0 0.0 _groundsearchdist)) (- _returnvalue (`KismetMathLibrary.MakeVector` 0.0 0.0 _groundsearchdist)) (`self.GroundSnapObjectTypes`) false (`local.ActorsToIgnore`) "None" true (struct :`R` 0.202823 :`G` 1.0 :`B` 0.456517 :`A` 1.0) (struct :`G` 1.0 :`B` 0.053794 :`A` 1.0)))
        (bind (_bblockinghit _binitialoverlap _time _distance _location) (`GameplayStatics.BreakHitResult` _outhit))
        (if _bblockinghit
          (`SplineComponent.SetLocationAtSplinePoint` _spline _index _location "World" true))))))

(fn `UserConstructionScript`
  (`parent.UserConstructionScript`)
  (if (`self.bSnapSplineToGround`)
    (`self.SnapSplineToGround`)))