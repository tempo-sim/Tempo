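; Proxy actor that describes a walkable strip along the left or right edge of its parent Tempo road to the road module queries.
; It stores no spline, reading the parent actor's spline and road width and offsetting positions sideways by half-widths plus RoadEdgeOffset.
; It reports two opposing "Walkable" lanes, and requests zone shapes only when WalkableWidth is positive.
; For Left, the distance-based right vector is negated, but the control-point one is not.
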(fn `GetDistanceAlongTempoRoadModuleAtControlPoint`
  (params (ControlPointIndex :type Integer))
  (returns (ReturnValue :type "Float (single-precision)"))
  (return (`SplineComponent.GetDistanceAlongSplineAtSplinePoint` (`self.GetParentSpline`) ControlPointIndex)))

(fn `GetDistanceAlongTempoRoadModuleClosestToWorldLocation`
  (params (QueryLocation :type "Vector Structure"))
  (returns (ReturnValue :type "Float (single-precision)"))
  (return (`SplineComponent.GetDistanceAlongSplineAtLocation` (`self.GetParentSpline`) QueryLocation "World")))

(fn `GetLocationAtDistanceAlongTempoRoadModule`
  (params (DistanceAlongRoadModule :type "Float (single-precision)") (CoordinateSpace :type "ETempoCoordinateSpace Enum" :default "Local"))
  (returns (ReturnValue :type "Vector Structure"))
  (bind _returnvalue (`/TempoAgents/Utilities/SplineFunctionLibrary.GetTempoLocationAtDistanceAlongSpline` (`self.GetParentSpline`) (`local.DistanceAlongRoadModule`) (`local.CoordinateSpace`)))
  (bind _returnvalue_2 (* (`/TempoAgents/Utilities/SplineFunctionLibrary.GetTempoRightVectorAtDistanceAlongSpline` (`self.GetParentSpline`) (`local.DistanceAlongRoadModule`) (`local.CoordinateSpace`)) (+ (/ (`self.GetParentRoadWidth`) 2.0) (`self.RoadEdgeOffset`) (/ (`self.WalkableWidth`) 2.0))))
  (switch `ETempoRoadLateralDirection` (`self.Direction`)
    (:`Left`
      (return (- _returnvalue _returnvalue_2)))
    (:`Right`
      (return (+ _returnvalue _returnvalue_2)))))

(fn `GetNumTempoRoadModuleControlPoints`
  (returns (ReturnValue :type Integer))
  (return (`SplineComponent.GetNumberOfSplinePoints` (`self.GetParentSpline`))))

(fn `GetNumTempoRoadModuleLanes`
  (returns (ReturnValue :type Integer))
  (return 2))

(fn `GetParentRoadWidth`
  (returns (Width :type "Float (double-precision)"))
  (bind _astempo_road_interface (cast `TempoRoadInterface` (`self.GetParentActor`)))
  (return (`TempoRoadInterface.GetTempoRoadWidth` _astempo_road_interface)))

(fn `GetParentSpline`
  (returns (Spline :type "SplineComponent Object Reference"))
  (return (`self.GetComponentByClass` (`self.GetParentActor`) "/Script/Engine.SplineComponent")))

(fn `GetRightVectorAtDistanceAlongTempoRoadModule`
  (params (DistanceAlongRoadModule :type "Float (single-precision)") (CoordinateSpace :type "ETempoCoordinateSpace Enum" :default "Local"))
  (returns (ReturnValue :type "Vector Structure"))
  (bind _returnvalue (`/TempoAgents/Utilities/SplineFunctionLibrary.GetTempoRightVectorAtDistanceAlongSpline` (`self.GetParentSpline`) DistanceAlongRoadModule CoordinateSpace))
  (switch `ETempoRoadLateralDirection` (`self.Direction`)
    (:`Left`
      (return (`KismetMathLibrary.NegateVector` _returnvalue)))
    (:`Right`
      (return _returnvalue))))

(fn `GetRotationAtDistanceAlongTempoRoadModule`
  (params (DistanceAlongRoadModule :type "Float (single-precision)") (CoordinateSpace :type "ETempoCoordinateSpace Enum" :default "Local"))
  (returns (ReturnValue :type "Rotator Structure"))
  (return (`/TempoAgents/Utilities/SplineFunctionLibrary.GetTempoRotationAtDistanceAlongSpline` (`self.GetParentSpline`) DistanceAlongRoadModule CoordinateSpace)))

(fn `GetTangentAtDistanceAlongTempoRoadModule`
  (params (DistanceAlongRoadModule :type "Float (single-precision)") (CoordinateSpace :type "ETempoCoordinateSpace Enum" :default "Local"))
  (returns (ReturnValue :type "Vector Structure"))
  (return (`/TempoAgents/Utilities/SplineFunctionLibrary.GetTempoTangentAtDistanceAlongSpline` (`self.GetParentSpline`) DistanceAlongRoadModule CoordinateSpace)))

(fn `GetTempoRoadModuleControlPointLocation`
  (params (ControlPointIndex :type Integer) (CoordinateSpace :type "ETempoCoordinateSpace Enum" :default "Local"))
  (returns (ReturnValue :type "Vector Structure"))
  (bind _returnvalue (`/TempoAgents/Utilities/SplineFunctionLibrary.GetTempoControlPointLocation` (`self.GetParentSpline`) ControlPointIndex CoordinateSpace))
  (bind _returnvalue_2 (* (`/TempoAgents/Utilities/SplineFunctionLibrary.GetTempoControlPointRightVector` (`self.GetParentSpline`) (`local.ControlPointIndex`) (`local.CoordinateSpace`)) (+ (/ (`self.GetParentRoadWidth`) 2.0) (`self.RoadEdgeOffset`) (/ (`self.WalkableWidth`) 2.0))))
  (switch `ETempoRoadLateralDirection` (`self.Direction`)
    (:`Left`
      (return (- _returnvalue _returnvalue_2)))
    (:`Right`
      (return (+ _returnvalue _returnvalue_2)))))

(fn `GetTempoRoadModuleControlPointRightVector`
  (params (ControlPointIndex :type Integer) (CoordinateSpace :type "ETempoCoordinateSpace Enum" :default "Local"))
  (returns (ReturnValue :type "Vector Structure"))
  (return (`/TempoAgents/Utilities/SplineFunctionLibrary.GetTempoControlPointRightVector` (`self.GetParentSpline`) ControlPointIndex CoordinateSpace)))

(fn `GetTempoRoadModuleControlPointRotation`
  (params (ControlPointIndex :type Integer) (CoordinateSpace :type "ETempoCoordinateSpace Enum" :default "Local"))
  (returns (ReturnValue :type "Rotator Structure"))
  (return (`/TempoAgents/Utilities/SplineFunctionLibrary.GetTempoControlPointRotation` (`self.GetParentSpline`) ControlPointIndex CoordinateSpace)))

(fn `GetTempoRoadModuleControlPointTangent`
  (params (ControlPointIndex :type Integer) (CoordinateSpace :type "ETempoCoordinateSpace Enum" :default "Local"))
  (returns (ReturnValue :type "Vector Structure"))
  (return (`/TempoAgents/Utilities/SplineFunctionLibrary.GetTempoControlPointTangent` (`self.GetParentSpline`) ControlPointIndex CoordinateSpace)))

(fn `GetTempoRoadModuleControlPointUpVector`
  (params (ControlPointIndex :type Integer) (CoordinateSpace :type "ETempoCoordinateSpace Enum" :default "Local"))
  (returns (ReturnValue :type "Vector Structure"))
  (return (`/TempoAgents/Utilities/SplineFunctionLibrary.GetTempoControlPointUpVector` (`self.GetParentSpline`) ControlPointIndex CoordinateSpace)))

(fn `GetTempoRoadModuleLaneDirection`
  (params (LaneIndex :type Integer))
  (returns (ReturnValue :type "EZoneLaneDirection Enum"))
  (if (< LaneIndex (/ (`self.GetNumTempoRoadModuleLanes`) 2))
    (return "Backward")
    (else
      (return "Forward"))))

(fn `GetTempoRoadModuleLaneProfileOverrideName`
  (returns (ReturnValue :type Name))
  (return "None"))

(fn `GetTempoRoadModuleLaneTags`
  (params (LaneIndex :type Integer))
  (returns (ReturnValue :type "Array of Name"))
  (return (`|MakeArray` "Walkable" :!type "Name")))

(fn `GetTempoRoadModuleLaneWidth`
  (params (LaneIndex :type Integer))
  (returns (ReturnValue :type "Float (single-precision)"))
  (return (/ (`self.WalkableWidth`) 2.0)))

(fn `GetTempoRoadModuleLength`
  (returns (ReturnValue :type "Float (single-precision)"))
  (return (`SplineComponent.GetSplineLength` (`self.GetParentSpline`))))

(fn `GetTempoRoadModuleParentActor`
  (returns (ReturnValue :type "Actor Object Reference"))
  (return (`self.GetParentActor`)))

(fn `GetTempoRoadModuleSampleDistanceStepSize`
  (returns (ReturnValue :type "Float (single-precision)"))
  (return (`self.SampleDistanceStepSize`)))

(fn `GetTempoRoadModuleWidth`
  (returns (ReturnValue :type "Float (single-precision)"))
  (return (`self.WalkableWidth`)))

(fn `GetUpVectorAtDistanceAlongTempoRoadModule`
  (params (DistanceAlongRoadModule :type "Float (single-precision)") (CoordinateSpace :type "ETempoCoordinateSpace Enum" :default "Local"))
  (returns (ReturnValue :type "Vector Structure"))
  (return (`/TempoAgents/Utilities/SplineFunctionLibrary.GetTempoUpVectorAtDistanceAlongSpline` (`self.GetParentSpline`) DistanceAlongRoadModule CoordinateSpace)))

(fn `IsTempoRoadModuleClosedLoop`
  (returns (ReturnValue :type Boolean))
  (return (`SplineComponent.IsClosedLoop` (`self.GetParentSpline`))))

(fn `ShouldGenerateZoneShapesForTempoRoadModule`
  (returns (ReturnValue :type Boolean))
  (return (> (`self.WalkableWidth`) 0.0)))

(fn `UserConstructionScript`)